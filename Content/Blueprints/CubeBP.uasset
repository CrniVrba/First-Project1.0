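; CubeBP is a player-controlled cube that is pushed along by physics impulses.
; On BeginPlay it adds the CubeInput Enhanced Input mapping context and starts a fast looping timer.
; The timer calls MoveCube, which applies a forward X velocity-change impulse to the Cube.
; The MoveInteraction action calls AddImpulse with no impulse wired in, leaving its value scaling unconnected.
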(event `self.ReceiveBeginPlay`
  (bind _asplayer_controller (cast `PlayerController` (`self.GetController`)))
  (bind _returnvalue (pcsubsystem `EnhancedInputLocalPlayerSubsystem` _asplayer_controller))
  (`/Engine/EditorBlueprintResources/StandardMacros.IsValid` _returnvalue
    (:`Is Valid`
      (`EnhancedInputSubsystemInterface.AddMappingContext` _returnvalue "/Game/Input/CubeInput.CubeInput" 0 (struct))
      (`KismetSystemLibrary.K2_SetTimerDelegate` (delegate `Move Cube`) 0.1 true))))

(event `Move Cube`
  (`PrimitiveComponent.AddImpulse` (`self.Cube`) (`KismetMathLibrary.MakeVector` (`self.Forward Impulse`)) "None" true))

(event `EnhancedInput|/Game/Input/MoveInteraction`
  (params (ActionValue :type "Float (double-precision)") (ElapsedSeconds :type "Float (double-precision)") (TriggeredSeconds :type "Float (double-precision)") (InputAction :type "InputAction Object Reference" :default "/Game/Input/MoveInteraction.MoveInteraction"))
  (:`Triggered`
    (`PrimitiveComponent.AddImpulse` (`self.Cube`) (0.0 0.0 0.0) "None" false)))

(fn `UserConstructionScript`)